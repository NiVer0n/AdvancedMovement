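; BP_AdvancedMovementCameraManager is a player camera manager that gives the advanced movement character an over-the-shoulder third-person view.
; Its BlueprintUpdateCamera override casts the view target to BP_AdvancedMovementCharacter and places the camera at a fixed offset behind, right of and above it.
; The offset and rotation follow player 0's control rotation, with no spring arm or collision check, and FOV comes from GetFOVAngle.
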(event EventBeginPlay)

(event Collision|EventActorBeginOverlap
  (params (OtherActor :type Actor%20Object%20Reference)))

(event EventTick
  (params (DeltaSeconds :type Float%20%28single-precision%29)))

(fn ConstructionScript)

(fn BlueprintUpdateCamera
  (params (CameraTarget :type Actor%20Object%20Reference))
  (bind _returnvalue (Game|GetPlayerController 0))
  (bind _returnvalue_2 (Pawn|GetControlRotation _returnvalue :!class /Script/Engine.Controller))
  (bind _asbp_advanced_movement_character (Utilities|Casting|CastToBP_AdvancedMovementCharacter CameraTarget))
  (return (+ (Transformation|GetActorLocation _asbp_advanced_movement_character) (+ (* (Math|Vector|GetForwardVector _returnvalue_2) -2.1e+02) (* (Math|Vector|GetRightVector _returnvalue_2) 45.0)) "0.000000,0.000000,60.000000") _returnvalue_2 (Camera|GetFOVAngle) true))